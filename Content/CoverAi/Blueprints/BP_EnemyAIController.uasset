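; BP_EnemyAIController is the AI controller that starts the StateTree logic for cover-AI enemies once they are ready.
; A looping timer from BeginPlay retries until the controlled BP_EnemyCharacter has a valid GunMesh and the player character exists.
; It then sets the player as the enemy's TargetActor, clears the timer and starts the StateTree, with a Started flag guarding against repeats.
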(event `self.ReceiveBeginPlay`
  (bind _returnvalue (`KismetSystemLibrary.K2_SetTimerDelegate` (delegate `TryStartAI`) 0.2 true))
  (set `self.StartTimer` _returnvalue))

(event `TryStartAI`
  (bind _returnvalue (`GameplayStatics.GetPlayerCharacter` 0))
  (if (not (`self.Started`))
    (bind _asbp_enemy_character (cast `/Game/CoverAi/Blueprints/BP_EnemyCharacter` (`self.K2_GetPawn`)))
    (if (`KismetSystemLibrary.IsValid` (`/Game/CoverAi/Blueprints/BP_EnemyCharacter.GunMesh` _asbp_enemy_character))
      (if (`KismetSystemLibrary.IsValid` _returnvalue)
        (set `/Game/CoverAi/Blueprints/BP_EnemyCharacter.TargetActor` _returnvalue _asbp_enemy_character)
        (set `self.Started` true)
        (`KismetSystemLibrary.K2_ClearAndInvalidateTimerHandle` (`self.StartTimer`))
        (`BrainComponent.StartLogic` (`self.StateTreeAI`))))))

(fn `UserConstructionScript`)
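; Enemy character for cover AI that carries a BP_Gun and shoots projectiles at its TargetActor.
; BeginPlay spawns the gun on the right hand socket, and Tick fires every frame that a muzzle-to-target visibility trace is clear, with no cooldown.
; Helper functions, not called here, yaw the body toward the target, measure muzzle height, and test cover by tracing from target eyes to a protected height above the feet.
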(event `self.ReceiveBeginPlay`
  (bind _returnvalue (`|SpawnActorFromClass` "/Game/CoverAi/Blueprints/BP_Gun.BP_Gun_C" (`SceneComponent.GetSocketTransform` (`self.Mesh`) "HandGrip_R" "RTS_World") "Undefined" "MultiplyWithRoot" self self))
  (set `self.GunMesh` _returnvalue)
  (bind _gunmesh (`self.GunMesh`)
    (:`then`
      (`self.K2_AttachToComponent` _gunmesh (`self.Mesh`) "HandGrip_R" "SnapToTarget" "SnapToTarget" "KeepWorld" false)
      (`PrimitiveComponent.IgnoreActorWhenMoving` (`self.CapsuleComponent`) (`self.GetOwner`) true))
    (:`else`)))

(event `self.ReceiveTick`
  (params (DeltaSeconds :type "Float (single-precision)"))
  (`self.FireProjectile`))

(fn `CanShoot`
  (returns (Allowed :type Boolean))
  (bind _gunmesh (`self.GunMesh`))
  (if (`KismetSystemLibrary.IsValid` _gunmesh)
    (bind (_aimlocation _valid) (`self.GetAimLocation`))
    (if _valid
      (bind (_outhit _returnvalue) (`KismetSystemLibrary.LineTraceSingle` (`SceneComponent.K2_GetComponentLocation` (`/Game/CoverAi/Blueprints/BP_Gun.MuzzlePoint` _gunmesh)) _aimlocation "TraceTypeQuery1"))
      (return (not _returnvalue))
      (else
        _)))
  (return false))

(fn `FaceTarget`
  (bind (_aimlocation _valid) (`self.GetAimLocation`))
  (if _valid
    (bind (_returnvalue_roll _returnvalue_pitch _returnvalue_yaw) (`KismetMathLibrary.BreakRotator` (`KismetMathLibrary.FindLookAtRotation` (`self.K2_GetActorLocation`) _aimlocation)))
    (`self.K2_SetActorRotation` (`KismetMathLibrary.MakeRotator` 0.0 0.0 _returnvalue_yaw))))

(fn `FireProjectile`
  (returns (Success :type Boolean))
  (bind _returnvalue (`SceneComponent.K2_GetComponentLocation` (`/Game/CoverAi/Blueprints/BP_Gun.MuzzlePoint` (`self.GunMesh`))))
  (bind _allowed (`self.CanShoot`))
  (if _allowed
    (bind (_aimlocation _valid) (`self.GetAimLocation`))
    (if _valid
      (`|SpawnActorFromClass` "/Game/CoverAi/Projectiles/BP_Projectile.BP_Projectile_C" (`KismetMathLibrary.MakeTransform` _returnvalue (`KismetMathLibrary.FindLookAtRotation` _returnvalue _aimlocation)) "AdjustIfPossibleButDontSpawnIfColliding" "MultiplyWithRoot" self self)
      (else
        (return false)))
    (else
      (return false))))

(fn `GetAimLocation`
  (returns (AimLocation :type "Vector Structure") (Valid :type Boolean))
  (bind _targetactor (`self.TargetActor`))
  (bind _returnvalue (`KismetSystemLibrary.IsValid` _targetactor))
  (if _returnvalue
    (return (`self.GetActorEyesViewPoint` _targetactor) true)
    (else
      (return (0.0 0.0 0.0) false))))

(fn `GetFeetLocation`
  (returns (FeetLocation :type "Vector Structure"))
  (return (- (`self.K2_GetActorLocation`) (`KismetMathLibrary.MakeVector` 0.0 0.0 (`CapsuleComponent.GetScaledCapsuleHalfHeight` (`self.CapsuleComponent`))))))

(fn `GetMuzzleHeight`
  (returns (Height :type "Float (double-precision)"))
  (bind (_returnvalue_x _returnvalue_y _returnvalue_z) (`KismetMathLibrary.BreakVector` (`SceneComponent.K2_GetComponentLocation` (`/Game/CoverAi/Blueprints/BP_Gun.MuzzlePoint` (`self.GunMesh`)))))
  (bind _feetlocation (`self.GetFeetLocation`))
  (return (- _returnvalue_z (.z _feetlocation))))

(fn `IsProtected`
  (returns (Protected :type Boolean))
  (bind _feetlocation (`self.GetFeetLocation`))
  (bind (_aimlocation _valid) (`self.GetAimLocation`))
  (if _valid
    (bind (_outhit _returnvalue) (`KismetSystemLibrary.LineTraceSingle` _aimlocation (+ _feetlocation (`KismetMathLibrary.MakeVector` 0.0 0.0 (`self.ProtectedHeight`))) "TraceTypeQuery1"))
    (return _returnvalue)
    (else
      (return false))))

(fn `UserConstructionScript`
  (bind _returnvalue (`GameplayStatics.GetActorOfClass` "/Game/CoverAi/Blueprints/BP_Gun.BP_Gun_C"))
  (set `self.GunMesh` _returnvalue))
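; BP_Projectile is a projectile in the CoverAi folder that damages only player-controlled characters.
; On BeginPlay its sphere collision ignores the owner while moving.
; The first hit on a non-owner actor sets a HasHit guard, applies a small fixed damage if that actor is a player-controlled Character, and destroys the projectile whatever was struck.
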(event `self.ReceiveBeginPlay`
  (`PrimitiveComponent.IgnoreActorWhenMoving` (`self.SphereCollision`) (`self.GetOwner`) true))

(event `self.SphereCollision.OnComponentHit`
  (params (HitComponent :type "PrimitiveComponent Object Reference") (OtherActor :type "Actor Object Reference") (OtherComp :type "PrimitiveComponent Object Reference") (NormalImpulse :type "Vector Structure") (Hit :type "HitResult Structure (by ref)"))
  (if (not (`self.bHasHit`))
    (if (!= OtherActor (`self.GetOwner`))
      (set `self.bHasHit` true)
      (bind _ascharacter (cast `Character` OtherActor)
        (:`then`
          (if (`Pawn.IsPlayerControlled` _ascharacter)
            (`GameplayStatics.ApplyDamage` _ascharacter 5.0 null self)))
        (:`CastFailed`
          _))
      (`self.K2_DestroyActor`))))

(fn `UserConstructionScript`)